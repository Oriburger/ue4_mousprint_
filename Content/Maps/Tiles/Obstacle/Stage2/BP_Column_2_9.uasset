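; BP_Column_2_9 is a Stage 2 column obstacle that shuttles its BPLaser1 component back and forth between Point1 and Point2.
; Each Tick, a Flag selects the target point and flips once the laser is within tolerance of it.
; Otherwise, MoveActorTo sets the laser's world location a fixed step along the look-at direction, without sweep or delta-time scaling, so speed depends on frame rate.
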(event `self.ReceiveTick`
  (params (DeltaSeconds :type "Float (single-precision)"))
  (bind _returnvalue (`SceneComponent.K2_GetComponentLocation` (`self.point2`)))
  (bind _returnvalue_2 (`SceneComponent.K2_GetComponentLocation` (`self.BP_Laser1`)))
  (bind _returnvalue_3 (`SceneComponent.K2_GetComponentLocation` (`self.BP_Laser1`)))
  (bind _returnvalue_4 (`SceneComponent.K2_GetComponentLocation` (`self.point1`)))
  (if (`self.flag`)
    (if (== _returnvalue_3 _returnvalue_4 :`ErrorTolerance` 5.0)
      (set `self.flag` false)
      (else
        (`self.Move Actor To` (`self.BP_Laser1`) (+ _returnvalue_3 (* (`KismetMathLibrary.GetForwardVector` (`KismetMathLibrary.FindLookAtRotation` _returnvalue_3 _returnvalue_4)) 7.0)))))
    (elif (== _returnvalue_2 _returnvalue :`ErrorTolerance` 5.0)
      (set `self.flag` true)
      (else
        (`self.Move Actor To` (`self.BP_Laser1`) (+ _returnvalue_2 (* (`KismetMathLibrary.GetForwardVector` (`KismetMathLibrary.FindLookAtRotation` _returnvalue_2 _returnvalue)) 7.0)))))))

(fn `Move Actor To`
  (params (Target :type "ChildActorComponent Object Reference") (NewLocation :type "Vector Structure"))
  (`SceneComponent.K2_SetWorldLocation` Target NewLocation false false))

(fn `UserConstructionScript`)