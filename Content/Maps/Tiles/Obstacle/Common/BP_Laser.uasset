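; BP_Laser is a destructible tile obstacle that takes three projectile hits to destroy and awards score.
; A hit on its Cube from an actor tagged Projectile advances StateLevel, turning the material yellow, then red.
; The third hit spawns an explosion effect and sound, adds points to the Score in BP_MainGameMode and destroys the actor.
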(event `self.Cube.OnComponentHit`
  (params (HitComponent :type "PrimitiveComponent Object Reference") (OtherActor :type "Actor Object Reference") (OtherComp :type "PrimitiveComponent Object Reference") (NormalImpulse :type "Vector Structure") (Hit :type "HitResult Structure (by ref)"))
  (bind _cube (`self.Cube`))
  (bind _returnvalue (`SceneComponent.K2_GetComponentLocation` (`self.RootComponent`)))
  (if (`self.ActorHasTag` OtherActor "Projectile")
    (switch `int` (`self.State Level`)
      (:`0`
        (`PrimitiveComponent.SetMaterial` _cube 0 "/Game/Test/E_Yellow.E_Yellow")
        (set `self.State Level` 1))
      (:`1`
        (`PrimitiveComponent.SetMaterial` _cube 0 "/Game/Test/E_Red.E_Red")
        (set `self.State Level` 2))
      (:`2`
        (`GameplayStatics.SpawnEmitterAtLocation` "/Game/StarterContent/Particles/P_Explosion.P_Explosion" _returnvalue)
        (`GameplayStatics.PlaySoundAtLocation` "/Game/StarterContent/Audio/Explosion01.Explosion01" _returnvalue (struct) 1.0 1.0 0.0 null null null)
        (bind _asbp_main_game_mode (cast `/Game/BP_MainGameMode` (`GameplayStatics.GetGameMode`)))
        (set `MainGameModeBase.Score` (+ (`MainGameModeBase.Score` _asbp_main_game_mode) 100.0) _asbp_main_game_mode)
        (`self.K2_DestroyActor`)))))

(fn `UserConstructionScript`)