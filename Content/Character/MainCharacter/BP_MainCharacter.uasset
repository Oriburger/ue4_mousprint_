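; Main character Blueprint that drives itself forward every tick and reflects lost health through post-processing.
; Each tick it also rebuilds the post-process settings, with one value growing as current HP falls relative to max HP.
; Holding C reattaches the following camera to a back boom, and releasing returns it to the normal boom, using a zero-time component move after each switch.
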(event `self.ReceiveTick`
  (params (DeltaSeconds :type "Float (single-precision)"))
  (`self.MoveForward` 1.0)
  (`self.UpdatePostProcess`))

(event `Key|C`
  (params (Key :type "Key Structure"))
  (bind _followingcamera (`self.FollowingCamera`))
  (:`Pressed`
    (`SceneComponent.K2_AttachToComponent` _followingcamera (`self.Camera Boom Back`) "None" "KeepWorld" "KeepWorld" "KeepWorld" true)
    (`KismetSystemLibrary.MoveComponentTo` _followingcamera (0.0 0.0 0.0) (struct) true true 0.0 :!label _label))
  (:`Released`
    (`SceneComponent.K2_AttachToComponent` _followingcamera (`self.CameraBoomNormal`) "None" "KeepWorld" "KeepWorld" "KeepWorld" true)
    (goto _label)))

(fn `UpdatePostProcess`
  (set `PostProcessComponent.Settings` (make `PostProcessSettings` :`SceneFringeIntensity` (* (- 1.0 (/ (`self.CharacterCurrHP`) (`self.CharacterMaxHP`))) 2.5)) (`self.PostProcess`)))

(fn `UserConstructionScript`)