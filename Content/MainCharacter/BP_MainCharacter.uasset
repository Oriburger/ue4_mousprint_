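; BP_MainCharacter is the main character Blueprint, which treats physics simulation on its mesh as the character's death.
; Each Tick prints the max walk speed as a debug readout and checks whether the mesh is simulating physics.
; The first time it is, a DoOnce clears IsInGame on BP_GameModeBase and prints a red "Die" message.
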(event `self.ReceiveTick`
  (params (DeltaSeconds :type "Float (single-precision)"))
  (`KismetSystemLibrary.PrintString` (`KismetStringLibrary.Conv_DoubleToString` (`self.CharacterMaxWalkSpeed`)) true true (struct :`G` 0.66 :`B` 1.0 :`A` 1.0) 0.001)
  (if (`SceneComponent.IsSimulatingPhysics` (`self.Mesh`) "None")
    (`/Engine/EditorBlueprintResources/StandardMacros.DoOnce` false
      (:`Completed`
        (bind _asbp_game_mode_base (cast `/Game/BP_GameModeBase` (`GameplayStatics.GetGameMode`)))
        (set `/Game/BP_GameModeBase.IsInGame` false _asbp_game_mode_base)
        (`KismetSystemLibrary.PrintString` "Die" true true (struct :`R` 1.0 :`G` 0.012011 :`A` 1.0) 10.0)))))

(fn `UserConstructionScript`)