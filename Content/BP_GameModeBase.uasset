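; Game mode that keeps a running survival score for the player.
; BeginPlay caches the player character as BP_MainCharacter.
; Tick then adds to Score in proportion to elapsed time for as long as that character reports it is not dead.
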(event `self.ReceiveBeginPlay`
  (bind _asbp_main_character (cast `/Game/MainCharacter/BP_MainCharacter` (`GameplayStatics.GetPlayerCharacter` 0)))
  (set `self.As BP Main Character` _asbp_main_character))

(event `self.ReceiveTick`
  (params (DeltaSeconds :type "Float (single-precision)"))
  (if (not (`MainCharacter.GetPlayerIsDead` (`self.As BP Main Character`)))
    (set `self.Score` (+ (* DeltaSeconds 10.0) (`self.Score`)))))

(fn `UserConstructionScript`)