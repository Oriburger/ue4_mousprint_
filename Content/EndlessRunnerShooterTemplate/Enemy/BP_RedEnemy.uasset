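; BP_RedEnemy is an enemy for the endless runner shooter that reacts to the player's approach and to being killed.
; It plays a crouch-to-idle stand-up animation when the player enters its warning area, and directly kills the player on reaching its fire area.
; On death, its skeletal mesh switches to physics ragdoll and receives a scaled impulse at the hit location.
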(event `self.OnDied`
  (params (hitImpulse :type "Vector Structure") (hitLocation :type "Vector Structure"))
  ;[1 1 1] Activate ragdoll on dead
  (`PrimitiveComponent.SetSimulatePhysics` (`self.SkeletalMesh`) true)
  (`PrimitiveComponent.AddImpulseAtLocation` (`self.SkeletalMesh`) (* hitImpulse 10000.0) hitLocation "None"))

(event `self.PlayerOnWarningArea`
  (params (EndlessRunnerShooterBase :type "/Game/EndlessRunnerShooterTemplate/Player/BP_EndlessRunnerShooterPawnBase Object Reference"))
  ;[1 1 1] When stand up animation when player enters warning area
  (`SkeletalMeshComponent.PlayAnimation` (`self.SkeletalMesh`) "/Game/EndlessRunnerShooterTemplate/StarterContent/Mannequin/Animations/ThirdPerson_CrouchToIdle.ThirdPerson_CrouchToIdle" false))

(event `self.PlayerOnFireArea`
  (params (endlessRunnerShooterBase :type "/Game/EndlessRunnerShooterTemplate/Player/BP_EndlessRunnerShooterPawnBase Object Reference"))
  ;[1 1 1] Shoot when player is in fire area
  (`/Game/EndlessRunnerShooterTemplate/Player/BP_EndlessRunnerShooterPawnBase.Die` endlessRunnerShooterBase))

(fn `UserConstructionScript`
  (`parent.UserConstructionScript`))