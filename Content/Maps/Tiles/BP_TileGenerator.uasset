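; Tile generator actor that keeps a sequence of BP_Tile_01 actors going in the level.
; On BeginPlay it spawns the first tile at InitialSpawnTransform and records it as the current tile.
; Tick polls CanSpawnTile; when true, it clears the flag, spawns a tile at GetNextSpawnTransform, calls DestroyPrevTile and makes the new tile current.
; Nothing in this file sets the flag to true.
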(event `self.ReceiveBeginPlay`
  (bind _returnvalue (`|SpawnActorFromClass` "/Game/Maps/Tiles/Blueprint/BP_Tile_01.BP_Tile_01_C" (`self.Initial Spawn Transform`) "Undefined" "OverrideRootScale" null null))
  (`self.SetCurrTile` _returnvalue))

(event `self.ReceiveTick`
  (params (DeltaSeconds :type "Float (single-precision)"))
  (if (`self.bCanSpawnTile`)
    (set `self.bCanSpawnTile` false)
    (bind _returnvalue (`|SpawnActorFromClass` "/Game/Maps/Tiles/Blueprint/BP_Tile_01.BP_Tile_01_C" (`self.GetNextSpawnTransform`) "Undefined" "OverrideRootScale" null null))
    (`self.DestroyPrevTile`)
    (`self.SetCurrTile` _returnvalue)))

(fn `UserConstructionScript`)