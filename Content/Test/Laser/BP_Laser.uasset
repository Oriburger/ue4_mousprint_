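; BP_Laser is a destructible laser hazard that damages the player and awards score when destroyed.
; Tick line-traces along the Arrow, moving the Niagara beam end and impact effect to the hit.
; Player-tagged hits trigger burn sound, hit-reaction montage and damage, throttled by a DoOnce reset after a short delay.
; Projectile hits on the Cube advance StateLevel through warning materials, then explode it and add to the game mode's Score.
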(event `self.ReceiveBeginPlay`
  (`FXSystemComponent.SetColorParameter` (`self.NiagaraLaser`) "Color" (struct :`G` 1.0 :`B` 0.094921 :`A` 0.01))
  (`FXSystemComponent.SetColorParameter` (`self.NiagaraLaserImpact`) "Color" (struct :`G` 1.0 :`B` 0.094921 :`A` 0.01)))

(event `self.ReceiveTick`
  (params (DeltaSeconds :type "Float (single-precision)"))
  (bind _returnvalue (`self.K2_GetActorLocation`))
  (bind _returnvalue_2 (+ _returnvalue (* (`SceneComponent.GetForwardVector` (`self.Arrow`)) (`self.Distance`))))
  (bind _outhit (`KismetSystemLibrary.LineTraceSingle` _returnvalue _returnvalue_2 "TraceTypeQuery2"))
  (bind (_bblockinghit _binitialoverlap _time _distance _location _impactpoint _normal _impactnormal _physmat _hitactor) (`GameplayStatics.BreakHitResult` _outhit))
  (`FXSystemComponent.SetVectorParameter` (`self.NiagaraLaser`) "LaserEnd" (select `bool` _bblockinghit :`false` _returnvalue_2 :`true` _location))
  (`SceneComponent.K2_SetWorldLocation` (`self.NiagaraLaserImpact`) _location false true)
  (`/Engine/EditorBlueprintResources/StandardMacros.IsValid` _hitactor
    (:`Is Valid`
      (if (`self.ActorHasTag` _hitactor "Player")
        (`/Engine/EditorBlueprintResources/StandardMacros.DoOnce` false :!label _label
          (:`Completed`
            (`GameplayStatics.PlaySoundAtLocation` "/Game/Test/Laser/SQ_Burn.SQ_Burn" _location (struct) 1.0 1.0 0.0 null null null)
            (bind _asbp_main_character (cast `/Game/MainCharacter/BP_MainCharacter` _hitactor))
            (`Character.PlayAnimMontage` _asbp_main_character "/Game/MainCharacter/Animation/Montage/Hit_Reaction_Montage.Hit_Reaction_Montage" 1.0 "None")
            (`GameplayStatics.ApplyDamage` _asbp_main_character 20.0 (`self.GetInstigatorController`) self)
            (`KismetSystemLibrary.Delay` 0.2)
            (goto _label :!via `Reset`)))))))

(event `self.Cube.OnComponentHit`
  (params (HitComponent :type "PrimitiveComponent Object Reference") (OtherActor :type "Actor Object Reference") (OtherComp :type "PrimitiveComponent Object Reference") (NormalImpulse :type "Vector Structure") (Hit :type "HitResult Structure (by ref)"))
  (bind _cube (`self.Cube`))
  (bind _returnvalue (`SceneComponent.K2_GetComponentLocation` (`self.RootComponent`)))
  (if (`self.ActorHasTag` OtherActor "Projectile")
    (switch `int` (`self.State Level`)
      (:`0`
        (`PrimitiveComponent.SetMaterial` _cube 0 "/Game/Test/E_Yellow.E_Yellow")
        (set `self.State Level` 1))
      (:`1`
        (`PrimitiveComponent.SetMaterial` _cube 0 "/Game/Test/E_Red.E_Red")
        (set `self.State Level` 2))
      (:`2`
        (`GameplayStatics.SpawnEmitterAtLocation` "/Game/StarterContent/Particles/P_Explosion.P_Explosion" _returnvalue)
        (`GameplayStatics.PlaySoundAtLocation` "/Game/StarterContent/Audio/Explosion01.Explosion01" _returnvalue (struct) 1.0 1.0 0.0 null null null)
        (bind _asbp_main_game_mode (cast `/Game/BP_MainGameMode` (`GameplayStatics.GetGameMode`)))
        (set `MainGameModeBase.Score` (+ (`MainGameModeBase.Score` _asbp_main_game_mode) 100.0) _asbp_main_game_mode)
        (`self.K2_DestroyActor`)))))

(fn `UserConstructionScript`)