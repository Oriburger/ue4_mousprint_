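; Laser obstacle actor that projects a beam and can be destroyed with two projectile hits.
; Each tick, a line trace sets the Niagara beam's end and impact effect position, falling back to 500 units along the arrow's forward vector.
; Sphere hits from actors tagged Projectile advance StateLevel: the first turns it red, the second spawns an explosion with sound and destroys the actor.
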(event `self.Sphere.OnComponentHit`
  (params (HitComponent :type "PrimitiveComponent Object Reference") (OtherActor :type "Actor Object Reference") (OtherComp :type "PrimitiveComponent Object Reference") (NormalImpulse :type "Vector Structure") (Hit :type "HitResult Structure (by ref)"))
  (bind _returnvalue (`SceneComponent.K2_GetComponentLocation` (`self.RootComponent`)))
  (if (`self.ActorHasTag` OtherActor "Projectile")
    (switch `int` (`self.State Level`)
      (:`0`
        (`PrimitiveComponent.SetMaterial` (`self.Sphere`) 0 "/Game/Test/E_Red.E_Red")
        (set `self.State Level` 1))
      (:`1`
        (`GameplayStatics.SpawnEmitterAtLocation` "/Game/Asset/StarterContent/Particles/P_Explosion.P_Explosion" _returnvalue)
        (`GameplayStatics.PlaySoundAtLocation` "/Game/Asset/StarterContent/Audio/Explosion01.Explosion01" _returnvalue (struct) 1.0 1.0 0.0 null null null null)
        (`self.K2_DestroyActor`)))))

(event `self.ReceiveTick`
  (params (DeltaSeconds :type "Float (single-precision)"))
  (bind _ns_laser (`self.NS_Laser`))
  (bind _ns_laserimpact (`self.NS_LaserImpact`))
  (bind _arrowcomponent (`self.ArrowComponent`))
  (bind _returnvalue (+ (`SceneComponent.K2_GetComponentLocation` _arrowcomponent) (* (`KismetMathLibrary.GetForwardVector` (`SceneComponent.K2_GetComponentRotation` _arrowcomponent)) 500.0)))
  (bind _returnvalue_2 (`self.GetLineTraceEndLocation`))
  (bind (_bblockinghit _binitialoverlap _time _distance _location) (`GameplayStatics.BreakHitResult` _returnvalue_2))
  (if _bblockinghit
    (`FXSystemComponent.SetVectorParameter` _ns_laser "LaserEnd" _location)
    (`SceneComponent.K2_SetWorldLocation` _ns_laserimpact _location false false)
    (else
      (`FXSystemComponent.SetVectorParameter` _ns_laser "LaserEnd" _returnvalue)
      (`SceneComponent.K2_SetWorldLocation` _ns_laserimpact _returnvalue false false))))

(fn `UserConstructionScript`)