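; BP_Tile_00 is a map tile that randomly populates itself with actors of a Target class when play begins.
; Eight sphere components serve as spawn points, each getting an independent coin flip on BeginPlay to decide whether an actor spawns at its world transform.
; The overlap and Tick events are empty, and the construction script does nothing.
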(event `self.ReceiveBeginPlay`
  (for _array_element (`|MakeArray` (`self.Sphere`) (`self.Sphere1`) (`self.Sphere2`) (`self.Sphere3`) (`self.Sphere4`) (`self.Sphere5`) (`self.Sphere7`) (`self.Sphere6`))
    (if (`KismetMathLibrary.RandomBool`)
      (`|SpawnActorFromClass` "/Game/Test/Target.Target_C" (`SceneComponent.K2_GetComponentToWorld` _array_element) "Undefined" "OverrideRootScale" null null))))

(fn `UserConstructionScript`)