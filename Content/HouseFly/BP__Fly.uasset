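; Housefly enemy that chases the player and self-destructs on getting close.
; A detection volume stores the Player-tagged actor as Target, and Tick turns and moves the fly toward it.
; The attack volume ramps emissive on dynamic materials, then explodes with effect and sound; the final character cast applies no damage.
; Hits from GameTraceChannel1 objects mark it dead, enable ragdoll physics and fade opacity before destruction.
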(event `self.ReceiveBeginPlay`
  (`self.SpawnDefaultController`))

(event `self.CapsuleComponent.OnComponentHit`
  (params (HitComponent :type "PrimitiveComponent Object Reference") (OtherActor :type "Actor Object Reference") (OtherComp :type "PrimitiveComponent Object Reference") (NormalImpulse :type "Vector Structure") (Hit :type "HitResult Structure (by ref)"))
  (bind _mesh (`self.Mesh`))
  (if (`|EnumEquality` (`PrimitiveComponent.GetCollisionObjectType` OtherComp) "ECC_GameTraceChannel1")
    (`PrimitiveComponent.SetSimulatePhysics` (`self.Mesh`) true)
    (set `self.IsDead` true)
    (`NavMovementComponent.StopActiveMovement` (`self.CharacterMovement`))
    (bind _returnvalue (`PrimitiveComponent.CreateDynamicMaterialInstance` _mesh 0 "/Game/Character_Appearance_Dissolve/Materials/Standart/BODY_Inst.BODY_Inst" "None"))
    (`PrimitiveComponent.SetMaterial` _mesh 0 _returnvalue)
    (bind _returnvalue_2 (`PrimitiveComponent.CreateDynamicMaterialInstance` _mesh 1 "/Game/Character_Appearance_Dissolve/Materials/Standart/WING_INST.WING_INST" "None"))
    (`PrimitiveComponent.SetMaterial` _mesh 1 _returnvalue_2)
    (bind (_direction `_새_트랙_0`) (`Timeline|타임라인_0`)
      (:`Update`
        (`MaterialInstanceDynamic.SetScalarParameterValue` _returnvalue "Opacity" `_새_트랙_0`)
        (`MaterialInstanceDynamic.SetScalarParameterValue` _returnvalue_2 "Opacity" `_새_트랙_0`))
      (:`Finished`
        (`self.K2_DestroyActor`)))))

(event `self.ReceiveTick`
  (params (DeltaSeconds :type "Float (single-precision)"))
  (bind _target (`self.Target`))
  (bind _returnvalue (`KismetMathLibrary.FindLookAtRotation` (`SceneComponent.K2_GetComponentLocation` (`self.CapsuleComponent`)) (`self.K2_GetActorLocation` _target)))
  (`/Engine/EditorBlueprintResources/StandardMacros.IsValid` _target
    (:`Is Valid`
      (`self.AddMovementInput` (`KismetMathLibrary.GetForwardVector` _returnvalue) 20.0)
      (`self.K2_SetActorRotation` _returnvalue))))

(event `self.PlayerDetectVolume.OnComponentBeginOverlap`
  (params (OverlappedComponent :type "PrimitiveComponent Object Reference") (OtherActor :type "Actor Object Reference") (OtherComp :type "PrimitiveComponent Object Reference") (OtherBodyIndex :type Integer) (bFromSweep :type Boolean) (SweepResult :type "HitResult Structure (by ref)"))
  (if (`self.ActorHasTag` OtherActor "Player")
    (set `self.Target` OtherActor)))

(event `self.PlayerAtkVolume.OnComponentBeginOverlap`
  (params (OverlappedComponent :type "PrimitiveComponent Object Reference") (OtherActor :type "Actor Object Reference") (OtherComp :type "PrimitiveComponent Object Reference") (OtherBodyIndex :type Integer) (bFromSweep :type Boolean) (SweepResult :type "HitResult Structure (by ref)"))
  (bind _returnvalue (`self.K2_GetActorLocation`))
  (bind _mesh (`self.Mesh`))
  (if (and (`self.ActorHasTag` OtherActor "Player") (not (`self.IsDead`)))
    (bind _returnvalue_2 (`PrimitiveComponent.CreateDynamicMaterialInstance` _mesh 0 "/Game/HouseFly/0_BODY.0_BODY" "None"))
    (`PrimitiveComponent.SetMaterial` _mesh 0 _returnvalue_2)
    (bind _returnvalue_3 (`PrimitiveComponent.CreateDynamicMaterialInstance` _mesh 1 "/Game/Character_Appearance_Dissolve/Materials/Standart/0_WING.0_WING" "None"))
    (`PrimitiveComponent.SetMaterial` _mesh 1 _returnvalue_3)
    (bind (_direction `_새_트랙_0`) (`Timeline|타임라인_1`)
      (:`Update`
        (`MaterialInstanceDynamic.SetScalarParameterValue` _returnvalue_2 "Emmisive" `_새_트랙_0`)
        (`MaterialInstanceDynamic.SetScalarParameterValue` _returnvalue_3 "Emmisive" `_새_트랙_0`))
      (:`Finished`
        (`GameplayStatics.SpawnEmitterAtLocation` "/Game/StarterContent/Particles/P_Explosion.P_Explosion" _returnvalue)
        (`GameplayStatics.PlaySoundAtLocation` "/Game/StarterContent/Audio/Explosion_Cue.Explosion_Cue" _returnvalue (struct) 1.0 1.0 0.0 null null null)
        (cast `/Game/MainCharacter/BP_MainCharacter` OtherActor
          (:`then`
            _)
          (:`CastFailed`
            _))
        (`self.K2_DestroyActor`)))))

(fn `UserConstructionScript`)